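; Mushroom boss that follows the player along the X axis and fires projectiles at them.
; Tick flips it to face the player while alive and adds movement input whenever the horizontal gap is at least 450 units.
; A looping timer, its interval randomized once at BeginPlay, jumps the animation state machine to the attack node.
; A separate Attack event aims the spawn point at the player and spawns BP_BossProjectile.
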(event `HandleRotation`
  (bind _returnvalue_x (`KismetMathLibrary.BreakVector` (`KismetMathLibrary.GetDirectionUnitVector` (`self.K2_GetActorLocation` (`GameplayStatics.GetPlayerCharacter` 0)) (`self.K2_GetActorLocation`))))
  ;[1 1 1] Handle rotation
  (if (`self.IsDead?`)
    _
    (elif (< _returnvalue_x 0.0)
      (`self.K2_SetActorRotation` (struct)) ; If true, Mushroom is facing right
      (else
        (`self.K2_SetActorRotation` (struct :`Yaw` 180.0)) ; If false Mushroom is facing left
      ))))

(event `self.ReceiveTick`
  (params (DeltaSeconds :type "Float (single-precision)"))
  (bind (_returnvalue_x _returnvalue_y _returnvalue_z) (`KismetMathLibrary.BreakVector` (- (`self.K2_GetActorLocation` (`GameplayStatics.GetPlayerCharacter` 0)) (`self.K2_GetActorLocation`))))
  (bind _returnvalue_x_2 (`KismetMathLibrary.BreakVector` (`KismetMathLibrary.Normal` (`KismetMathLibrary.MakeVector` _returnvalue_x _returnvalue_y _returnvalue_z))))
  ;[1 1 1] Boss Movement and rotation
  (`self.HandleRotation`)
  (if (not (< (`KismetMathLibrary.Abs` _returnvalue_x) 450.0))
    (`self.AddMovementInput` (1.0 0.0 0.0) _returnvalue_x_2)))

(event `self.ReceiveBeginPlay`
  (bind _returnvalue (`KismetSystemLibrary.K2_SetTimerDelegate` (delegate `PlayBossAttackAnimation`) (`KismetMathLibrary.RandomFloatInRange` 2.0 4.0) true))
  (set `self.BossAttackEvent` _returnvalue))

(event `PlayBossAttackAnimation`
  (`PaperZDAnimInstance.JumpToNode` (`PaperZDAnimationComponent.AnimInstance` (`self.AnimationComponent`)) "BossAttack" "None"))

(event `Attack`
  (`SceneComponent.K2_SetWorldRotation` (`self.ProjectileSpawn`) (`KismetMathLibrary.FindLookAtRotation` (`self.K2_GetActorLocation`) (`self.K2_GetActorLocation` (`GameplayStatics.GetPlayerCharacter` 0))) false false)
  (`|SpawnActorFromClass` "/Game/Boss/Blueprints/BP_BossProjectile.BP_BossProjectile_C" (`SceneComponent.K2_GetComponentToWorld` (`self.ProjectileSpawn`)) "Undefined" "MultiplyWithRoot" null null))

(fn `UserConstructionScript`)