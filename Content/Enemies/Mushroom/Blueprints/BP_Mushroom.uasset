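; Mushroom ranged enemy that turns to face the player along X and fires BP_Projectile from a spawn point.
; The player entering its box starts a looping timer that jumps to the attack animation; a separate event spawns the projectile.
; Damage updates a widget health bar, then either knocks the mushroom back with a hit animation or plays death, switches capsule collision and destroys it after a delay.
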(event `self.ReceiveBeginPlay`
  ;[1 1 1] Initialise Health and Widgets
  (set `self.MaxHealth` (`self.Health`)) ; Set Mushroom health
  (bind _aswb_ranged_enemy_health_bar (cast `/Game/WidgetBlueprints/WB_RangedEnemyHealthBar` (`WidgetComponent.GetWidget` (`self.Widget`))))
  (bind _output_get (set `self.As WB Ranged Enemy Health Bar` _aswb_ranged_enemy_health_bar))
  (set `/Game/WidgetBlueprints/WB_RangedEnemyHealthBar.MushroomRef` self _output_get))

(event `self.ReceiveTick`
  (params (DeltaSeconds :type "Float (single-precision)"))
  (`self.HandleRotation`))

(event `HandleRotation`
  (bind _returnvalue_x (`KismetMathLibrary.BreakVector` (`KismetMathLibrary.GetDirectionUnitVector` (`self.K2_GetActorLocation` (`GameplayStatics.GetPlayerCharacter` 0)) (`self.K2_GetActorLocation`))))
  ;[1 1 1] Mushroom is always facing character
  (if (`self.IsDead?`)
    _
    (elif (< _returnvalue_x 0.0)
      (`self.K2_SetActorRotation` (struct)) ; If true, Mushroom is facing right
      (else
        (`self.K2_SetActorRotation` (struct :`Yaw` 180.0)) ; If false Mushroom is facing left
      ))))

(event `self.ReceiveAnyDamage`
  (params (Damage :type "Float (single-precision)") (DamageType :type "DamageType Object Reference") (InstigatedBy :type "Controller Object Reference") (DamageCauser :type "Actor Object Reference"))
  (bind _returnvalue_x (`KismetMathLibrary.BreakVector` (`KismetMathLibrary.GetDirectionUnitVector` (`self.K2_GetActorLocation` DamageCauser) (`self.K2_GetActorLocation`))))
  ;[1 1 1] Mushroom take damage system
  (set `self.Health` (- (`self.Health`) Damage))
  (`/Game/WidgetBlueprints/WB_RangedEnemyHealthBar.Update Healthbar` (`self.As WB Ranged Enemy Health Bar`))
  (set `self.EnemyDamaged?` true)
  (if (<= (`self.Health`) 0.0)
    (`PaperZDAnimInstance.JumpToNode` (`PaperZDAnimationComponent.AnimInstance` (`self.AnimationComponent`)) (`self.MushroomDeathNode`) "None")
    (set `self.IsDead?` true)
    (`SceneComponent.SetVisibility` (`self.Widget`) false false)
    (`PrimitiveComponent.SetCollisionProfileName` (`self.CapsuleComponent`) "OverlapOnlyPawn" true)
    (`KismetSystemLibrary.Delay` 3.0)
    (`self.K2_DestroyActor`)
    (else
      (`self.LaunchCharacter` (`KismetMathLibrary.MakeVector` (* (select `bool` (< _returnvalue_x 0.0) :`false` -1.0 :`true` 1.0) -800.0) 0.0 150.0) true true) ; Launch character when hit
      (`PaperZDAnimInstance.JumpToNode` (`PaperZDAnimationComponent.AnimInstance` (`self.AnimationComponent`)) (`self.DamagedJumpNode`) "None")
      (`SceneComponent.SetVisibility` (`self.Widget`) true false)
      (`KismetSystemLibrary.RetriggerableDelay` 1.0)
      (set `self.EnemyDamaged?` false))))

(event `self.Box.OnComponentBeginOverlap`
  (params (OverlappedComponent :type "PrimitiveComponent Object Reference") (OtherActor :type "Actor Object Reference") (OtherComp :type "PrimitiveComponent Object Reference") (OtherBodyIndex :type Integer) (bFromSweep :type Boolean) (SweepResult :type "HitResult Structure (by ref)"))
  ;[1 0.4938 0.0916] Mushroom ranged attack system
  ;;[1 1 1] Projectile Damage the player
  (if (== OtherActor (`GameplayStatics.GetPlayerCharacter` 0))
    (`KismetSystemLibrary.K2_SetTimerDelegate` (delegate `MushroomAttack`) 1.0 true)))

(event `MushroomAttack`
  ;[1 0.4938 0.0916] Mushroom ranged attack system
  ;;[1 1 1] Projectile Damage the player
  (if (not (`self.IsDead?`))
    (`PaperZDAnimInstance.JumpToNode` (`PaperZDAnimationComponent.AnimInstance` (`self.AnimationComponent`)) (`self.RangedAttackJumpNode`) "None")))

(event `SpawnProjectile`
  ;[1 0.4938 0.0916] Mushroom ranged attack system
  ;;[1 1 1] Spawn Mushroom Projectile
  (`|SpawnActorFromClass` "/Game/Enemies/Mushroom/Blueprints/BP_Projectile.BP_Projectile_C" (`KismetMathLibrary.MakeTransform` (`SceneComponent.K2_GetComponentLocation` (`self.ProjectileSpawnPoint`)) (`self.K2_GetActorRotation`)) "Undefined" "MultiplyWithRoot" null null))

(fn `UserConstructionScript`)