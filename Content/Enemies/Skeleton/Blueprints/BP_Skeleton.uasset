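; Side-scrolling skeleton enemy that patrols along the X axis, attacks the player and takes damage.
; Forward and downward traces detect walls and ledges, pausing it before it reverses.
; Player overlap with the box loops a timed attack animation, while a separate Attack event traces forward to deal damage.
; Hits update the health bar, turn it toward the attacker and knock it back; death plays an animation, then destroys it.
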(event `self.ReceiveBeginPlay`
  ;[1 1 1] initialise health and widgets
  (set `CharacterMovementComponent.MaxWalkSpeed` (`self.Max Walk Speed`) (`self.CharacterMovement`))
  (set `self.MaxHealth` (`self.Health`))
  (bind _aswb_enemy_health_bar (cast `/Game/WidgetBlueprints/WB_EnemyHealthBar` (`WidgetComponent.GetWidget` (`self.Widget`))))
  (set `/Game/WidgetBlueprints/WB_EnemyHealthBar.SkeletonReference` self _aswb_enemy_health_bar)
  (set `self.As WB Enemy Health Bar` _aswb_enemy_health_bar))

(event `self.ReceiveTick`
  (params (DeltaSeconds :type "Float (single-precision)"))
  ;[1 1 1] Every tick handle this
  (`self.HandleRotation`)
  (`self.HandleMovement`))

(event `HandleMovement`
  (bind _returnvalue (`self.K2_GetActorLocation`))
  (bind _returnvalue_2 (`self.K2_GetActorLocation`))
  ;[1 1 1] Skeleton Wall Detection
  (if (not (`self.IsDead?`))
    (`self.AddMovementInput` (1.0 0.0 0.0) (`self.MovementDirection`))
    (`|ExecutionSequence`
      (:`then_0`
        (bind (_outhit _returnvalue_3) (`KismetSystemLibrary.LineTraceSingleForObjects` _returnvalue (+ _returnvalue (* (`self.GetActorForwardVector`) (100.0 0.0 0.0))) (`|MakeArray` "ObjectTypeQuery1" "ObjectTypeQuery2" "ObjectTypeQuery3" :!type "EObjectTypeQuery Enum") false (`|MakeArray` (`GameplayStatics.GetPlayerCharacter` 0) :!type "Actor Object Reference"))) ; Look for these objects and ignore these actors
        (if _returnvalue_3
          (`/Engine/EditorBlueprintResources/StandardMacros.DoOnce` false :!label _label
            (:`Completed`
              (set `CharacterMovementComponent.MaxWalkSpeed` 0.0 (`self.CharacterMovement`))
              (`KismetSystemLibrary.Delay` (`self.WaitTime`))
              (set `CharacterMovementComponent.MaxWalkSpeed` (`self.Max Walk Speed`) (`self.CharacterMovement`))
              (set `self.MovementDirection` (* (`self.MovementDirection`) -1.0))
              (goto _label :!via `Reset`)))))
      (:`then_1`
        ;[1 1 1] Ledge Detection
        (bind (_outhit_2 _returnvalue_4) (`KismetSystemLibrary.LineTraceSingleForObjects` _returnvalue_2 (+ (- _returnvalue_2 (0.0 0.0 150.0)) (* (`self.GetActorForwardVector`) (100.0 0.0 0.0))) (`|MakeArray` "ObjectTypeQuery1" "ObjectTypeQuery2" "ObjectTypeQuery3" :!type "EObjectTypeQuery Enum") false (`|MakeArray` (`GameplayStatics.GetPlayerCharacter` 0) :!type "Actor Object Reference"))) ; Look for these objects and ignore these actors
        (if (not _returnvalue_4)
          (goto _label))))))

(event `HandleRotation`
  ;[1 1 1] Skeleton Rotation
  (if (> (`self.MovementDirection`) 0.0)
    (`self.K2_SetActorRotation` (struct))
    (else
      (`self.K2_SetActorRotation` (struct :`Yaw` 180.0)))))

(event `self.ReceiveAnyDamage`
  (params (Damage :type "Float (single-precision)") (DamageType :type "DamageType Object Reference") (InstigatedBy :type "Controller Object Reference") (DamageCauser :type "Actor Object Reference"))
  (bind _returnvalue_x (`KismetMathLibrary.BreakVector` (`KismetMathLibrary.GetDirectionUnitVector` (`self.K2_GetActorLocation` DamageCauser) (`self.K2_GetActorLocation`))))
  (bind _returnvalue (select `bool` (< _returnvalue_x 0.0) :`false` -1.0 :`true` 1.0))
  ;[1 1 1] Skeleton take damage system
  (set `self.Health` (- (`self.Health`) Damage))
  (`/Game/WidgetBlueprints/WB_EnemyHealthBar.Update Healthbar` (`self.As WB Enemy Health Bar`))
  (set `self.EnemyDamaged?` true)
  (set `self.MovementDirection` _returnvalue)
  (if (<= (`self.Health`) 0.0)
    (`PaperZDAnimInstance.JumpToNode` (`PaperZDAnimationComponent.AnimInstance` (`self.AnimationComponent`)) (`self.DeathJumpNode`) "None")
    (set `self.IsDead?` true)
    (`SceneComponent.SetVisibility` (`self.Widget`) false false)
    (`PrimitiveComponent.SetCollisionProfileName` (`self.CapsuleComponent`) "OverlapOnlyPawn" true)
    (`KismetSystemLibrary.Delay` 3.0)
    (`self.K2_DestroyActor`)
    (else
      (`self.LaunchCharacter` (`KismetMathLibrary.MakeVector` (* _returnvalue -800.0) 0.0 150.0) true true) ; Launch character when hit
      (`PaperZDAnimInstance.JumpToNode` (`PaperZDAnimationComponent.AnimInstance` (`self.AnimationComponent`)) (`self.DamagedJumpNode`) "None")
      (`SceneComponent.SetVisibility` (`self.Widget`) true false)
      (`KismetSystemLibrary.RetriggerableDelay` 1.0)
      (set `self.EnemyDamaged?` false))))

(event `self.Box.OnComponentBeginOverlap`
  (params (OverlappedComponent :type "PrimitiveComponent Object Reference") (OtherActor :type "Actor Object Reference") (OtherComp :type "PrimitiveComponent Object Reference") (OtherBodyIndex :type Integer) (bFromSweep :type Boolean) (SweepResult :type "HitResult Structure (by ref)"))
  ;[1 1 1] Skeleton Attack
  (if (== OtherActor (`GameplayStatics.GetPlayerCharacter` 0))
    (set `self.AttackMode` true)
    (bind _returnvalue (`KismetSystemLibrary.K2_SetTimerDelegate` (delegate `SkeletonAttack`) 1.0 true)) ; Every 1 second call the Jump to node for AttackEvent for skeleton
    (set `self.AttackEvent` _returnvalue)))

(event `SkeletonAttack`
  ;[1 1 1] Skeleton Attack
  (if (not (`self.IsDead?`))
    (`PaperZDAnimInstance.JumpToNode` (`PaperZDAnimationComponent.AnimInstance` (`self.AnimationComponent`)) (`self.AttackJumpNode`) "None")))

(event `self.Box.OnComponentEndOverlap`
  (params (OverlappedComponent :type "PrimitiveComponent Object Reference") (OtherActor :type "Actor Object Reference") (OtherComp :type "PrimitiveComponent Object Reference") (OtherBodyIndex :type Integer))
  ;[1 1 1] Skeleton stop attacking
  (if (== OtherActor (`GameplayStatics.GetPlayerCharacter` 0))
    (set `self.AttackMode` false)
    (`KismetSystemLibrary.K2_ClearAndInvalidateTimerHandle` (`self.AttackEvent`))))

(event `Attack`
  (bind _returnvalue (`self.K2_GetActorLocation`))
  ;[1 1 1] Skeleton apply damage to player
  (bind _outhit (`KismetSystemLibrary.LineTraceSingleForObjects` _returnvalue (+ _returnvalue (* (`self.GetActorForwardVector`) (100.0 0.0 0.0))) (`|MakeArray` "ObjectTypeQuery3" :!type "EObjectTypeQuery Enum")))
  (bind (_bblockinghit _binitialoverlap _time _distance _location _impactpoint _normal _impactnormal _physmat _hitactor) (`GameplayStatics.BreakHitResult` _outhit))
  (if (== _hitactor (`GameplayStatics.GetPlayerCharacter` 0))
    (`GameplayStatics.ApplyDamage` _hitactor 1.0)))

(fn `UserConstructionScript`)