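; BP_CoinPickup is a coin that Player_BP collects by overlapping its Sphere component.
; Each pickup adds one to the player's Coins, refreshes the HUD coin count and destroys the actor.
; If the player already holds 100 coins, the pickup instead resets Coins to zero, grants a life and updates only the HUD lives display.
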(event `self.Sphere.OnComponentBeginOverlap`
  (params (OverlappedComponent :type "PrimitiveComponent Object Reference") (OtherActor :type "Actor Object Reference") (OtherComp :type "PrimitiveComponent Object Reference") (OtherBodyIndex :type Integer) (bFromSweep :type Boolean) (SweepResult :type "HitResult Structure (by ref)"))
  (bind _as_player_bp (`self.As Player BP`))
  (bind _as_player_bp_2 (`self.As Player BP`))
  (bind _asplayer_bp (cast `/Game/PlayerCharacter/Player_BP` OtherActor))
  (bind _output_get (set `self.As Player BP` _asplayer_bp))
  (if (== (`/Game/PlayerCharacter/Player_BP.Coins` _output_get) 100.0)
    ;[1 1 1] If player reaches 100 coins increase their lives by 1
    (set `/Game/PlayerCharacter/Player_BP.Coins` 0.0 _as_player_bp_2)
    (set `/Game/PlayerCharacter/Player_BP.Lives` (+ (`/Game/PlayerCharacter/Player_BP.Lives` _as_player_bp_2) 1.0) _as_player_bp_2)
    (`/Game/WidgetBlueprints/WB_PlayerHUD.UpdateLives` (`/Game/PlayerCharacter/Player_BP.HUD_Ref` _as_player_bp_2))
    (`self.K2_DestroyActor`)
    (else
      (set `/Game/PlayerCharacter/Player_BP.Coins` (+ (`/Game/PlayerCharacter/Player_BP.Coins` _as_player_bp) 1.0) _as_player_bp)
      (`/Game/WidgetBlueprints/WB_PlayerHUD.UpdateCoins` (`/Game/PlayerCharacter/Player_BP.HUD_Ref` _as_player_bp))
      (`self.K2_DestroyActor`))))

(fn `UserConstructionScript`)