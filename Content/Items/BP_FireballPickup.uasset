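; Fireball ammo pickup that restocks the player's fireballs when they overlap its sphere.
; If the player is not already at max, it adds a fixed amount clamped to the maximum, otherwise it stays in the world.
; On pickup it writes the new count into the player's save object, saves to slot immediately, refreshes the HUD and destroys itself.
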(event `self.Sphere.OnComponentBeginOverlap`
  (params (OverlappedComponent :type "PrimitiveComponent Object Reference") (OtherActor :type "Actor Object Reference") (OtherComp :type "PrimitiveComponent Object Reference") (OtherBodyIndex :type Integer) (bFromSweep :type Boolean) (SweepResult :type "HitResult Structure (by ref)"))
  (bind _as_player_bp (`self.As Player BP`))
  (bind _as_sg_save_game (`/Game/PlayerCharacter/Player_BP.As SG Save Game` (`self.As Player BP`)))
  ;[1 1 1] Frieblal pickup
  (bind _asplayer_bp (cast `/Game/PlayerCharacter/Player_BP` OtherActor))
  (bind _output_get (set `self.As Player BP` _asplayer_bp))
  (if (not (== (`/Game/PlayerCharacter/Player_BP.Fireballs` _output_get) (`/Game/PlayerCharacter/Player_BP.MaxFireballs` _output_get)))
    (bind _output_get_2 (set `/Game/PlayerCharacter/Player_BP.Fireballs` (`KismetMathLibrary.Clamp` (+ (`/Game/PlayerCharacter/Player_BP.Fireballs` _as_player_bp) 5) 1 (`/Game/PlayerCharacter/Player_BP.MaxFireballs` _as_player_bp)) _as_player_bp))
    (set `/Game/PlayerCharacter/SG_SaveGame.Fireballs` (`KismetMathLibrary.Conv_IntToDouble` _output_get_2) _as_sg_save_game)
    (`GameplayStatics.SaveGameToSlot` _as_sg_save_game "1")
    (`/Game/WidgetBlueprints/WB_PlayerHUD.UpdateFireballs` (`/Game/PlayerCharacter/Player_BP.HUD_Ref` (`self.As Player BP`)))
    (`self.K2_DestroyActor`)))

(fn `UserConstructionScript`)