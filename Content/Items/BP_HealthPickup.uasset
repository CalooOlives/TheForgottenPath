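; Health pickup actor that restores health to the player when touched.
; Its sphere overlap casts the other actor to Player_BP and does nothing if health is already at max.
; Otherwise it adds HealthToGive, clamps the result to max health, calls ShowHearts on the player's HUD with the truncated amount and destroys itself.
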(event `self.Sphere.OnComponentBeginOverlap`
  (params (OverlappedComponent :type "PrimitiveComponent Object Reference") (OtherActor :type "Actor Object Reference") (OtherComp :type "PrimitiveComponent Object Reference") (OtherBodyIndex :type Integer) (bFromSweep :type Boolean) (SweepResult :type "HitResult Structure (by ref)"))
  (bind _as_player_bp (`self.As Player BP`))
  ;[1 1 1] Pickup Health
  (bind _asplayer_bp (cast `/Game/PlayerCharacter/Player_BP` OtherActor))
  (bind _output_get (set `self.As Player BP` _asplayer_bp))
  (if (not (== (`/Game/PlayerCharacter/Player_BP.Health` _output_get) (`/Game/PlayerCharacter/Player_BP.MaxHealth` _output_get)))
    (set `/Game/PlayerCharacter/Player_BP.Health` (`KismetMathLibrary.FClamp` (+ (`/Game/PlayerCharacter/Player_BP.Health` _as_player_bp) (`self.HealthToGive`)) 1.0 (`/Game/PlayerCharacter/Player_BP.MaxHealth` _as_player_bp)) _as_player_bp)
    (`/Game/WidgetBlueprints/WB_PlayerHUD.ShowHearts` (`/Game/PlayerCharacter/Player_BP.HUD_Ref` (`self.As Player BP`)) (`KismetMathLibrary.FTrunc` (`self.HealthToGive`)))
    (`self.K2_DestroyActor`)))

(fn `UserConstructionScript`)