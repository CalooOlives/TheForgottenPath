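; BP_MovingSaw is a moving saw hazard that damages actors it touches.
; The construction script gives InterpToMovement two relative control points, Location1 and Location2, to move between.
; The Speed variable sets the movement's Duration, so higher values mean slower travel.
; A Sphere component's begin-overlap event applies a small fixed damage to any overlapping actor, with no filtering.
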(event `self.Sphere.OnComponentBeginOverlap`
  (params (OverlappedComponent :type "PrimitiveComponent Object Reference") (OtherActor :type "Actor Object Reference") (OtherComp :type "PrimitiveComponent Object Reference") (OtherBodyIndex :type Integer) (bFromSweep :type Boolean) (SweepResult :type "HitResult Structure (by ref)"))
  (`GameplayStatics.ApplyDamage` OtherActor 1.0))

(fn `UserConstructionScript`
  (bind _interptomovement (`self.InterpToMovement`))
  ;[1 1 1] Platform moving between points
  (set `InterpToMovementComponent.ControlPoints` (`|MakeArray` (make `InterpControlPoint` (`self.Location1`)) (make `InterpControlPoint` (`self.Location2`))) _interptomovement) ; Manually set control points
  (set `InterpToMovementComponent.Duration` (`self.Speed`) _interptomovement))