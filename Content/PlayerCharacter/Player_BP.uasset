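; Player character for a 2D side-scroller with dash, wall slide and jump, line-trace attack and limited fireballs.
; Enhanced Input drives movement and abilities, with DoOnce cooldowns and animation node jumps, while Tick flips facing from X velocity.
; BeginPlay loads lives, coins and fireballs from the save and creates the HUD.
; Damage shakes the camera and updates the HUD; death disables input, and Respawn spends a life at the checkpoint or shows game over.
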(event `self.ReceiveBeginPlay`
  ;[1 1 1] Initialise player HUD readings.
  (bind _returnvalue (`GameplayStatics.LoadGameFromSlot` "1"))
  (bind _assg_save_game (cast `/Game/PlayerCharacter/SG_SaveGame` _returnvalue))
  (bind _output_get (set `self.As SG Save Game` _assg_save_game))
  (set `self.Lives` (`/Game/PlayerCharacter/SG_SaveGame.Lives` _output_get))
  (set `self.Coins` (`/Game/PlayerCharacter/SG_SaveGame.Coins` _output_get))
  (set `self.Fireballs` (`KismetMathLibrary.FTrunc` (`/Game/PlayerCharacter/SG_SaveGame.Fireballs` _output_get))) ; Initialise all HUD collectibles
  (`WidgetBlueprintLibrary.SetInputMode_GameOnly` (`GameplayStatics.GetPlayerController` 0))
  (bind _asplayer_controller (cast `PlayerController` (`self.GetController`)))
  (bind _returnvalue_2 (pcsubsystem `EnhancedInputLocalPlayerSubsystem` _asplayer_controller))
  (`/Engine/EditorBlueprintResources/StandardMacros.IsValid` _returnvalue_2
    (:`Is Valid`
      (`EnhancedInputSubsystemInterface.AddMappingContext` _returnvalue_2 "/Game/Input/IMC_Default.IMC_Default" 0 (struct))
      (bind _returnvalue_3 (`|CreateWidget` "/Game/WidgetBlueprints/WB_PlayerHUD.WB_PlayerHUD_C"))
      (bind _output_get_2 (set `self.HUD_Ref` _returnvalue_3))
      (`UserWidget.AddToViewport` _output_get_2 0)
      (set `self.MaxHealth` (`self.Health`))
      (set `self.Checkpoint` (`self.K2_GetActorLocation`)))))

(event `EnhancedInput|/Game/Input/Actions/IA_Move`
  (params (ActionValue :type "Float (double-precision)") (ElapsedSeconds :type "Float (double-precision)") (TriggeredSeconds :type "Float (double-precision)") (InputAction :type "InputAction Object Reference" :default "/Game/Input/Actions/IA_Move.IA_Move"))
  ;[0.2541 0.5536 1] Player movement
  (:`Triggered`
    (if (> ActionValue 0.0)
      (set `self.MoveRight?` true)
      (elif (< ActionValue 0.0)
        (set `self.MoveRight?` false)))
    (`self.AddMovementInput` (1.0 0.0 0.0) ActionValue) ; only change Player's X direction axis
  ))

(event `self.ReceiveTick`
  (params (DeltaSeconds :type "Float (single-precision)"))
  (bind _returnvalue (`self.GetController`))
  (bind _returnvalue_2 (`self.GetController`))
  (bind _velocity_x (`KismetMathLibrary.BreakVector` (`MovementComponent.Velocity` (`self.CharacterMovement`))))
  ;[0.2541 0.5536 1] See if float value > 0  or < 0
  (`/Engine/EditorBlueprintResources/StandardMacros.CompareFloat` _velocity_x ; compare X velocity values
    (:`>`
      ;[0.2541 0.5536 1] Player rotating to the right
      (`/Engine/EditorBlueprintResources/StandardMacros.IsValid` _returnvalue_2 :!label _label
        (:`Is Valid`
          (`Controller.SetControlRotation` _returnvalue_2 (`KismetMathLibrary.MakeRotator` 0.0)))))
    (:`==`
      (if (`self.MoveRight?`)
        (goto _label)
        (else
          ;[0.2541 0.5536 1] Player rotating to the left
          (`/Engine/EditorBlueprintResources/StandardMacros.IsValid` _returnvalue :!label _label_2
            (:`Is Valid`
              (`Controller.SetControlRotation` _returnvalue (`KismetMathLibrary.MakeRotator` 0.0 0.0 180.0)))))))
    (:`<`
      (goto _label_2))))

(event `InputAction|Dash`
  (params (Key :type "Key Structure"))
  ;[1 1 1] Player Dash
  (:`Pressed`
    (`/Engine/EditorBlueprintResources/StandardMacros.DoOnce` false :!label _label_3
      (:`Completed`
        (`PaperZDAnimInstance.JumpToNode` (`PaperZDAnimationComponent.AnimInstance` (`self.AnimationComponent`)) "Dash" "None") ; Enter the jump node in animation sequence
        (if (`NavMovementComponent.IsFalling` (`self.CharacterMovement`))
          (set `CharacterMovementComponent.GravityScale` 0.0 (`self.CharacterMovement`)) ; prevent player from falling after dashing
        )
        (`self.LaunchCharacter` (`KismetMathLibrary.MakeVector` (select `bool` (`self.MoveRight?`) :`false` -3000.0 :`true` 3000.0)) true true)
        (`KismetSystemLibrary.Delay` 0.3)
        (set `CharacterMovementComponent.GravityScale` 1.0 (`self.CharacterMovement`)) ; reset gravity scale after 0.3 seconds
        (goto _label_3 :!via `Reset`)))))

(event `self.ReceiveHit`
  (params (MyComp :type "PrimitiveComponent Object Reference") (Other :type "Actor Object Reference") (OtherComp :type "PrimitiveComponent Object Reference") (bSelfMoved :type Boolean) (HitLocation :type "Vector Structure") (HitNormal :type "Vector Structure") (NormalImpulse :type "Vector Structure") (Hit :type "HitResult Structure (by ref)"))
  (bind _sprite (`self.Sprite`))
  (bind _sprite_2 (`self.Sprite`))
  (bind (_relativelocation_x _relativelocation_y _relativelocation_z) (`KismetMathLibrary.BreakVector` (`SceneComponent.RelativeLocation` _sprite)))
  (bind (_relativelocation_x_2 _relativelocation_y_2 _relativelocation_z_2) (`KismetMathLibrary.BreakVector` (`SceneComponent.RelativeLocation` _sprite_2)))
  ;[1 1 1] Player wall slide
  (if (and (`self.ActorHasTag` Other "Wall") (`NavMovementComponent.IsFalling` (`self.CharacterMovement`)))
    (set `self.WallSlide?` true)
    (`SceneComponent.K2_SetRelativeLocation` _sprite_2 (`KismetMathLibrary.MakeVector` 15.0 _relativelocation_y_2 _relativelocation_z_2) false false) ; 'latch' player onto a wall
    (`KismetSystemLibrary.RetriggerableDelay` 0.1) ; after 0.1 seconds set player condition to 'not on a wall'
    (set `self.WallSlide?` false)
    (`SceneComponent.K2_SetRelativeLocation` _sprite (`KismetMathLibrary.MakeVector` 0.0 _relativelocation_y _relativelocation_z) false false) ; 'release' player from the wall
  ))

(event `Attack`
  (bind _returnvalue (`self.K2_GetActorLocation`))
  ;[1 1 1] Attack Event
  (bind _outhit (`KismetSystemLibrary.LineTraceSingleForObjects` _returnvalue (+ _returnvalue (* (`self.GetActorForwardVector`) (100.0 0.0 0.0))) (`|MakeArray` "ObjectTypeQuery3" :!type "EObjectTypeQuery Enum") false (`|MakeArray` (`GameplayStatics.GetPlayerCharacter` 0) :!type "Actor Object Reference"))) ; Setup Line trace for player
  (`GameplayStatics.ApplyDamage` (`.HitActor` (`GameplayStatics.BreakHitResult` _outhit)) 1.0 null self) ; Player damage
)

(event `self.CapsuleComponent.OnComponentHit`
  (params (HitComponent :type "PrimitiveComponent Object Reference") (OtherActor :type "Actor Object Reference") (OtherComp :type "PrimitiveComponent Object Reference") (NormalImpulse :type "Vector Structure") (Hit :type "HitResult Structure (by ref)"))
  ;[1 0.9459 0.07549] TESTING
  (`KismetSystemLibrary.PrintString` "Level Complete!" (`self.ActorHasTag` OtherActor "LevelComplete")))

(event `InputAction|Jump`
  (params (Key :type "Key Structure"))
  (bind _returnvalue_x (`KismetMathLibrary.BreakVector` (`self.GetActorForwardVector`)))
  ;[0.2541 0.5536 1] Player Jump/wall jump
  (:`Pressed`
    (if (`self.WallSlide?`)
      (`self.LaunchCharacter` (`KismetMathLibrary.MakeVector` (* _returnvalue_x -1000.0) 0.0 750.0) true true) ; Launch character off wall when they're on the wall and pressed jump
      (else
        (`self.Jump`))))
  (:`Released`
    (`self.StopJumping`)))

(event `Key|One`
  (params (Key :type "Key Structure"))
  ;[0.4072 0.3813 0.03071] Damage Testing
  (:`Pressed`
    (`GameplayStatics.ApplyDamage` self 1.0)
    (`KismetSystemLibrary.PrintString` "Hello")))

(event `InputAction|Attack`
  (params (Key :type "Key Structure"))
  ;[1 1 1] Trigger Attack
  (:`Pressed`
    (`/Engine/EditorBlueprintResources/StandardMacros.DoOnce` false :!label _label_4
      (:`Completed`
        (`PaperZDAnimInstance.JumpToNode` (`PaperZDAnimationComponent.AnimInstance` (`self.AnimationComponent`)) "AttackEvent" "None")
        (`KismetSystemLibrary.Delay` 0.4)
        (goto _label_4 :!via `Reset`)))))

(event `self.ReceiveAnyDamage`
  (params (Damage :type "Float (single-precision)") (DamageType :type "DamageType Object Reference") (InstigatedBy :type "Controller Object Reference") (DamageCauser :type "Actor Object Reference"))
  ;[1 1 1] Player camera shake when player takes damage
  (set `self.Health` (- (`self.Health`) Damage))
  (`GameplayStatics.PlayWorldCameraShake` "/Game/PlayerCharacter/BP_DamagedCamShake.BP_DamagedCamShake_C" (`self.K2_GetActorLocation`) 0.0 1100.0)
  (for _ (range 1 (+ (`KismetMathLibrary.FTrunc` Damage) 1))
    (`/Game/WidgetBlueprints/WB_PlayerHUD.Player Damaged` (`self.HUD_Ref`)))
  (if (<= (`self.Health`) 0.0)
    (`/Engine/EditorBlueprintResources/StandardMacros.DoOnce` false :!label _label_5
      (:`Completed`
        (`self.DisableInput` (`GameplayStatics.GetPlayerController` 0)) ; Don't let player take control once dead
        (`PaperZDAnimInstance.JumpToNode` (`PaperZDAnimationComponent.AnimInstance` (`self.AnimationComponent`)) "BH_Death" "None") ; play death animation
        (`Widget.RemoveFromParent` (`self.HUD_Ref`)) ; Remove HUD from view when player dies
      ))))

(event `ResetPlayerDeath`
  ;[1 1 1] Player camera shake when player takes damage
  (goto _label_5 :!via `Reset`))

(event `InputAction|SpawnFireballProjectile`
  (params (Key :type "Key Structure"))
  ;[1 1 1] Launch Fireball projectile from the spawn point on the player
  (:`Pressed`
    (if (> (`self.Fireballs`) 0)
      (`/Engine/EditorBlueprintResources/StandardMacros.DoOnce` false :!label _label_6
        (:`Completed`
          (`|SpawnActorFromClass` "/Game/PlayerCharacter/BP_FireballProjectile.BP_FireballProjectile_C" (`KismetMathLibrary.MakeTransform` (`SceneComponent.K2_GetComponentLocation` (`self.FBSpawnPoint`)) (`self.K2_GetActorRotation`)) "Undefined" "MultiplyWithRoot" null null)
          (bind _result (`/Engine/EditorBlueprintResources/StandardMacros.DecrementInt` (`self.Fireballs`))
            (:`  `
              (set `self.Fireballs` _result)
              (`/Game/WidgetBlueprints/WB_PlayerHUD.UpdateFireballs` (`self.HUD_Ref`))
              (`KismetSystemLibrary.Delay` (`self.ProjectileResetTime`))
              (goto _label_6 :!via `Reset`))))))))

(event `Respawn`
  ;[0.2541 0.5536 1] Respawn player
  (if (> (`self.Lives`) 0.0)
    (set `self.Respawn?` true)
    (`self.EnableInput` (`GameplayStatics.GetPlayerController` 0)) ; Enable player controls again once respawned
    (set `self.Health` (`self.MaxHealth`)) ; give player's full health back
    (bind _result (`/Engine/EditorBlueprintResources/StandardMacros.DecrementFloat` (`self.Lives`))
      (:`  `
        (set `self.Lives` _result) ; Remove 1 life
        (bind _returnvalue (`|CreateWidget` "/Game/WidgetBlueprints/WB_PlayerHUD.WB_PlayerHUD_C"))
        (bind _output_get (set `self.HUD_Ref` _returnvalue))
        (`UserWidget.AddToViewport` _output_get 0)
        (`self.K2_SetActorLocation` (`self.Checkpoint`)) ; Spawn at interacted checkpoint
        (`self.ResetPlayerDeath`)))
    (else
      (set `self.Respawn?` false)
      (bind _returnvalue_2 (`|CreateWidget` "/Game/WidgetBlueprints/WB_GameOver.WB_GameOver_C"))
      (`UserWidget.AddToViewport` _returnvalue_2 0))))

(event `InputAction|Pause`
  (params (Key :type "Key Structure"))
  ;[1 1 1] Pause menu
  (:`Pressed`
    (bind _returnvalue (`|CreateWidget` "/Game/WidgetBlueprints/WB_PauseMenu.WB_PauseMenu_C"))
    (`UserWidget.AddToViewport` _returnvalue 0)))

(fn `UserConstructionScript`)